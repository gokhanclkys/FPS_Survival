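; BP_PatrolActor defines a patrol route as a spline and hands out its points one after another as patrol locations.
; ReturnNextPatrolLocation advances the stored patroller index, then returns that spline point's world-space position.
; The index lives on the actor and resets to zero only after equalling the point count, so it can step one past the last point.
; Event graph and construction script are empty.
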(event EventBeginPlay)

(event Collision|EventActorBeginOverlap
  (params (OtherActor :type Actor%20Object%20Reference)))

(event EventTick
  (params (DeltaSeconds :type Float%20%28single-precision%29)))

(fn ConstructionScript)

(fn ReturnNextPatrolLocation
  (CallFunction|IncreasePatrollerIndex)
  (return (Spline|GetLocationatSplinePoint (Variables|Default|GetSpline) (Variables|Default|GetCurrentPatrollerIndex) "World")))

(fn IncreasePatrollerIndex
  (if (== (Variables|Default|GetCurrentPatrollerIndex) (Spline|GetNumberOfSplinePoints (Variables|Default|GetSpline)))
    (Variables|Default|SetCurrentPatrollerIndex 0)
    (else
      (Math|Integer|IncrementInt (Variables|Default|GetCurrentPatrollerIndex)))))
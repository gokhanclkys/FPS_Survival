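; Arrow projectile that stops and sticks on its first hit.
; Until stuck, it line-traces each Tick between two arrowhead components, ignoring the player pawn, and disables mesh physics, gravity and collision on a hit.
; Any Character counts as an enemy: the arrow snaps to its mesh socket nearest the impact, keeping world rotation, and swaps visibility to the ArrowSticked component.
; Other hits leave it frozen in place.
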(event EventBeginPlay)

(event Collision|EventActorBeginOverlap
  (params (OtherActor :type Actor%20Object%20Reference)))

(event EventTick
  (params (DeltaSeconds :type Float%20%28single-precision%29))
  (if (not (Variables|Default|GetSticked))
    (bind (_hit _outhit) (CallFunction|TraceArrowHit))
    (if _hit
      (Development|PrintString "Hello")
      (bind (_notenemy _mesh _socketname) (CallFunction|CheckifHitEnemy (.ImpactPoint (Collision|BreakHitResult _outhit)) (.HitActor (Collision|BreakHitResult _outhit))))
      (if _notenemy
        (CallFunction|Nullify)
        (else
          (Components|SkeletalMesh|SetSkeletalMeshAsset (Variables|Default|GetSkeletalMesh) "/Game/Blueprints/PlayerAssets/SM_BowNG.SM_BowNG")
          (CallFunction|Nullify)
          (Transformation|AttachComponentToComponent _mesh _socketname "SnapToTarget" "KeepWorld" "KeepWorld" true)
          (CallFunction|ShowSM)))
      (Variables|Default|SetSticked true))))

(fn ConstructionScript)

(fn TraceArrowHit
  (bind (_outhit _returnvalue) (Collision|LineTraceByChannel (Transformation|GetWorldLocation (Variables|Default|GetArrowHead)) (Transformation|GetWorldLocation (Variables|Default|GetArrowHead2)) "TraceTypeQuery2" true (Utilities|Array|MakeArray (Game|Player|GetPlayerPawn 0)) "ForOneFrame"))
  (return _returnvalue _outhit))

(fn CheckifHitEnemy
  (params (ArrowHitLocation :type Vector) (Actor :type Object%20Object%20Reference))
  (bind _ascharacter (Utilities|Casting|CastToCharacter Actor)
    (:then
      (for _array_element (Transformation|GetAllSocketNames (Variables|/Script/Engine.Character|GetMesh _ascharacter))
        (Utilities|Array|Add (LocalVariables|GetDistances) (Math|Vector|Distance(Vector) ArrowHitLocation (Transformation|GetSocketLocation (Variables|/Script/Engine.Character|GetMesh _ascharacter) _array_element))))
      (return false (Variables|/Script/Engine.Character|GetMesh _ascharacter) (Utilities|Array|Get(acopy) (Transformation|GetAllSocketNames (Variables|/Script/Engine.Character|GetMesh _ascharacter)) (.IndexOfMinValue (Math|Float|MinOfFloatArray (LocalVariables|GetDistances))))))
    (:CastFailed
      (return true 0 "None"))))

(fn Nullify
  (Physics|SetSimulatePhysics (Variables|Default|GetSkeletalMesh) false)
  (Physics|SetEnableGravity (Variables|Default|GetSkeletalMesh) false)
  (Collision|SetCollisionEnabled (Variables|Default|GetSkeletalMesh) "NoCollision"))

(fn ShowSM
  (Development|SetHiddeninGame (Variables|Default|GetSkeletalMesh) true false)
  (Development|SetHiddeninGame (Variables|Default|GetArrowSticked) false false))
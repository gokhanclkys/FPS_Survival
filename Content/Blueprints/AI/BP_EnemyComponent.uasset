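; Actor component for enemy AI that tracks its owner's ground speed and holds an enemy state.
; It caches the owner's CharacterMovementComponent on BeginPlay, then computes horizontal velocity length every Tick, ignoring Z.
; SetWalkingAndIdleStates resets the state to the first enum entry at near-zero speed unless one protected state is active.
; That function has no walking branch and is not called within this Blueprint.
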(event EventBeginPlay
  (Variables|MovementComponent|SetCharacterMovementComponent (Actor|GetComponentbyClass (Components|GetOwner) "/Script/Engine.CharacterMovementComponent")))

(event EventTick
  (params (DeltaSeconds :type Float%20%28single-precision%29))
  (CallFunction|CalculateGroundSpeed))

(fn CalculateGroundSpeed
  (bind _charactermovementcomponent (Variables|MovementComponent|GetCharacterMovementComponent))
  (bind _velocity (Variables|/Script/Engine.MovementComponent|GetVelocity _charactermovementcomponent))
  (Utilities|IsValid _charactermovementcomponent
    (:Is%20Valid
      (Variables|MovementComponent|SetGroundSpeed (Math|Vector|VectorLength (Math|Vector|MakeVector (.x _velocity) (.y _velocity) 0.0))))))

(fn SetWalkingandIdleStates
  (if (not (> (Variables|MovementComponent|GetGroundSpeed) 1.0))
    (if (Utilities|Enum|NotEqual(Enum) (Variables|Default|GetE_EnemyState) "NewEnumerator2")
      (Variables|Default|SetE_EnemyState "NewEnumerator0"))))